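; BP_CrawlSpaceTrigger is a gameplay trigger volume, named for crawl spaces, that switches an animation state on the Hero.
; When the Hero begins overlapping the box, it sends a trigger animation message to the Hero's AI controller.
; When the Hero stops overlapping, it sends the matching end animation message with the same enum value.
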(event OnComponentBeginOverlap(BoxTrigger)
  (params (OverlappedComponent :type Primitive%20Component%20Object%20Reference) (OtherActor :type Actor%20Object%20Reference) (OtherComp :type Primitive%20Component%20Object%20Reference) (OtherBodyIndex :type Integer) (bFromSweep :type Boolean) (SweepResult :type Hit%20Result%20Structure%20%28by%20ref%29))
  (if (== OtherActor (Variables|Default|GetHero))
    (Class|BPIAnimationTrigger|TriggerAnimation(Message) (AI|GetAIController (Variables|Default|GetHero)) "NewEnumerator0")))

(event OnComponentEndOverlap(BoxTrigger)
  (params (OverlappedComponent :type Primitive%20Component%20Object%20Reference) (OtherActor :type Actor%20Object%20Reference) (OtherComp :type Primitive%20Component%20Object%20Reference) (OtherBodyIndex :type Integer))
  (if (== OtherActor (Variables|Default|GetHero))
    (Class|BPIAnimationTrigger|EndAnimation(Message) (AI|GetAIController (Variables|Default|GetHero)) "NewEnumerator0")))

(event EventBeginPlay)

(event Collision|EventActorBeginOverlap
  (params (OtherActor :type Actor%20Object%20Reference)))

(event EventTick
  (params (DeltaSeconds :type Float%20%28single-precision%29)))

(fn ConstructionScript)