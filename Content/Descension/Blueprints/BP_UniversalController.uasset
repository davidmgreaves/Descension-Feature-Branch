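; Player controller for touch tap-to-move navigation, where a single tap sneaks and a double tap runs.
; Each press traces under the finger and restarts a retriggerable delay, while releases before it ends count as taps.
; When the delay expires, movement stops, and a tap on a valid hit sets walk speed from the tap count and calls SimpleMoveToLocation to the hit point.
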(event EventBeginPlay
  (Class|PlayerController|ActivateTouchInterface))

(event Input|TouchEvents|InputTouch
  (params (Location :type Vector) (FingerIndex :type ETouchIndex%20Enum))
  (bind (_hitresult _returnvalue) (Class|PlayerController|GetHitResultUnderFingerbyChannel FingerIndex "TraceTypeQuery1" true))
  ;[1 1 1] Handle Navigation Tap Inputs
  (:Pressed
    (Variables|Default|SetHitResult _hitresult)
    (Variables|Default|SetHitResultIsValid _returnvalue)
    (Utilities|FlowControl|RetriggerableDelay (Variables|Default|GetTapDelay))
    (AI|Navigation|StopMovement)
    (Variables|Default|SetDelayHasEnded true)
    (if (Variables|Default|GetTouchWasTap)
      (if (Variables|Default|GetHitResultIsValid)
        (CallFunction|ResetInputChecks)
        (CallFunction|MovetoLocation)
        (Variables|Default|SetNumberOfTaps 0))
      (else
        (CallFunction|ResetInputChecks))))
  (:Released
    (if (not (Variables|Default|GetDelayHasEnded))
      (Variables|Default|SetTouchWasTap true)
      (bind _result (Math|Integer|IncrementInt (Variables|Default|GetNumberOfTaps))))))

(fn ConstructionScript)

(fn MovetoLocation
  ;[1 1 1] Moves the player to a location retrieved from the hit component at a speed determined by a single or double tap
  (switch int (Variables|Default|GetNumberOfTaps)
    (:1
      (Variables|/Script/Engine.CharacterMovementComponent|SetMaxWalkSpeed (Variables|/Script/Engine.Character|GetCharacterMovement (Game|GetPlayerCharacter 0)) (Variables|Default|GetSneakSpeed)))
    (:2
      (Variables|/Script/Engine.CharacterMovementComponent|SetMaxWalkSpeed (Variables|/Script/Engine.Character|GetCharacterMovement (Game|GetPlayerCharacter 0)) (Variables|Default|GetRunSpeed))))
  (bind _output_get (Variables|Default|SetDestination (.Location (Collision|BreakHitResult (Variables|Default|GetHitResult)))))
  (AI|Navigation|SimpleMovetoLocation self _output_get))

(fn ResetInputChecks
  (Variables|Default|SetTouchWasTap false)
  (Variables|Default|SetDelayHasEnded false)
  (Variables|Default|SetHitResultIsValid false))