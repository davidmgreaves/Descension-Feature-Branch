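; Behavior tree task for the patrol AI that records whether the player is currently sensed.
; It reads the player pawn's entry from the AIC_Patrol controller's AI perception and copies the first stimulus's successfully-sensed state into the IsVisible blackboard key.
; It also prints that stimulus location, then finishes successfully once the controller cast passes; a failed cast never finishes the task.
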(event EventReceiveExecute
  (params (OwnerActor :type Actor%20Object%20Reference))
  (bind _asaic_patrol (Utilities|Casting|CastToAIC_Patrol OwnerActor))
  (bind _info (Class|AIPerceptionComponent|GetActorsPerception (Variables|/Game/Descension/Blueprints/AI/AIC_Patrol.AIC_Patrol_C|GetAIPerception _asaic_patrol) (Game|Player|GetPlayerPawn 0)))
  (Development|PrintString (Utilities|String|ToString(Vector) (.StimulusLocation (Utilities|Struct|BreakAIStimulus (Utilities|Array|Get(acopy) (.LastSensedStimuli (Utilities|Struct|BreakActorPerceptionBlueprintInfo _info)))))))
  (if (.bSuccessfullySensed (Utilities|Struct|BreakAIStimulus (Utilities|Array|Get(acopy) (.LastSensedStimuli (Utilities|Struct|BreakActorPerceptionBlueprintInfo _info)))))
    (Class|BTFunctionLibrary|SetBlackboardValueasBool (Variables|Default|GetIsVisible) true)
    (else
      (Class|BTFunctionLibrary|SetBlackboardValueasBool (Variables|Default|GetIsVisible) false)))
  (AI|BehaviorTree|FinishExecute true))