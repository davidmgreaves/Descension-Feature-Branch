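; Touch player controller that views through BP_SpectatorCharacter and steers it indirectly via its AI controller.
; Timers and swipe length classify taps, double taps, presses and swipes: tap sneaks to the hit point, double tap switches to running, press calls StopMovement.
; The tapped component's collision object type selects an arrival action, fired when a timeline polling velocity detects a stop.
; Only TakeCover crouches; other arrival actions are print placeholders, Swipe is empty and QuickTurn is unused.
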(event Custom|SingleTap
  (bind _player_char_ref (Variables|Default|GetPLAYER_CHAR_Ref))
  (bind _hitresult (Variables|Default|GetHitResult))
  (bind (_bblockinghit _binitialoverlap _time _location _impactpoint _normal _impactnormal _physmat _hitactor _hitcomponent) (Collision|BreakHitResult _hitresult))
  ;[1 1 1] Single Tap Event
  (Variables|Default|SetDestination _impactpoint)
  (Variables|Default|SetHit%20Component _hitcomponent)
  (if (Math|Vector|Equal(Vector) (Transformation|GetActorLocation _hitactor) (Transformation|GetActorLocation (Variables|Default|GetPLAYER_CHAR_Ref)) 0.0001)
    (if (Variables|/Script/Engine.Character|GetbIsCrouched _player_char_ref)
      (Character|UnCrouch _player_char_ref))
    (else
      (CallFunction|SetPlayerSpeed (Variables|Default|GetSneakSpeed)) ; If not, then we want the player character to walk to the location of the Touch Input at walk speed
      (if (Variables|Default|GetHitResultIsValid)
        (CallFunction|MovetoLocation (Variables|Default|GetDestination) (Variables|Default|GetHit%20Component)) ; Move the player to the location stored inside our HitComponent variable
        (Variables|Default|SetHitResultIsValid false)
        (else
          (Development|PrintString "Hit Result is not valid"))))))

(event Custom|Swipe
  ;[1 1 1] Swipe Event
)

(event Custom|Press
  ;[1 1 1] Press Event
  (AI|Navigation|StopMovement))

(event Custom|Poll%20For%20End%20of%20Movement
  ;[1 1 1] Check if the player has reached their destination
  (Timeline|Poll%20For%20Arrival PlayFromStart
    (:Update
      (if (> (Math|Vector|VectorLength (Variables|/Script/Engine.MovementComponent|GetVelocity (Variables|/Script/Engine.Character|GetCharacterMovement (Variables|Default|GetPLAYER_CHAR_Ref)))) 0.0)
        (Variables|Default|SetIsInTransit true)
        (elif (Variables|Default|GetIsInTransit)
          (Variables|Default|SetIsInTransit false)
          (Utilities|FlowControl|DoOnce false :!label _label
            (:Completed
              (switch Utilities|FlowControl|Switch|SwitchonActorActionsAtDestination (Variables|Default|GetActionOnArrival)
                (:NewEnumerator4
                  _)
                (:NewEnumerator0
                  (CallFunction|TakeCover))
                (:NewEnumerator1
                  (CallFunction|HugWall))
                (:NewEnumerator2
                  (CallFunction|InteractwithObject))
                (:NewEnumerator3
                  (CallFunction|StealthTakeDown)))
              (Variables|Default|SetActionOnArrival "NewEnumerator4")
              (Timeline|Poll%20For%20Arrival Stop)))
          (else
            (goto _label Reset)))))))

(event Custom|DoubleTap
  (bind _player_char_ref (Variables|Default|GetPLAYER_CHAR_Ref))
  ;[1 1 1] Double Tap Event
  (if (Variables|/Script/Engine.Character|GetbIsCrouched _player_char_ref)
    (Character|UnCrouch _player_char_ref))
  (CallFunction|SetPlayerSpeed (Variables|Default|GetRunSpeed)) ; On aDouble Tap we want the player character to run to the desired location. MoveToLocation was already called on the first tap, calling it a second time would risk changing the characters desired location, instead of just their speed
)

(event Custom|Take%20Cover
  ;[1 1 1] Crouch Behind Cover
  (Development|PrintString "Take Cover!")
  (Character|Crouch (Variables|Default|GetPLAYER_CHAR_Ref)))

(event Custom|Hug%20Wall
  (Development|PrintString "Hug Wall")
  (Variables|Default|SetIsInTransit false))

(event Custom|Interact%20With%20Object
  (Development|PrintString "Interact with object"))

(event Custom|Stealth%20Take%20Down
  (Development|PrintString "Stealth Take Down!"))

(event EventBeginPlay
  ;[1 1 1] Set references to the AI driven Player Character and it's AI Controller, set render target of the Spectactors' camera to the Characters camera, and remove virtual joysticks from screen
  (bind _outactors (Actor|GetAllActorsOfClass "/Game/Descension/Blueprints/BP_SpectatorCharacter.BP_SpectatorCharacter_C"))
  (for _array_element _outactors
    (bind _output_get (Variables|Default|SetPLAYER_CHAR_Ref _array_element))
    (Variables|Default|SetAI_CON_REF (.AsBP%20Spectator%20AI%20CON (Utilities|Casting|CastToBP_SpectatorAI_CON (AI|GetAIController _output_get))))
    (Game|Player|SetViewTargetwithBlend (Variables|Default|GetPLAYER_CHAR_Ref) 0.0 "VTBlend_Linear" 0.0 false)
    (Class|PlayerController|ActivateTouchInterface)))

(event Input|TouchEvents|InputTouch
  (params (Location :type Vector) (FingerIndex :type ETouchIndex%20Enum))
  (bind (_hitresult _returnvalue) (Class|PlayerController|GetHitResultUnderFingerbyChannel FingerIndex "TraceTypeQuery1" false))
  (bind _returnvalue_2 (Game|GetPlayerController 0))
  (bind (_locationx _locationy) (Class|PlayerController|GetInputTouchState _returnvalue_2 "Touch1"))
  (bind _returnvalue_3 (Math|Vector2D|MakeVector2D _locationx _locationy))
  ;[1 1 1] Maps the possible Touch and Gesture Inputs with their corresponding Events
  (:Pressed
    (if _returnvalue
      (Variables|Default|SetHitResultIsValid true)
      (Variables|Default|SetHitResult _hitresult)
      (bind _output_get (Variables|Default|SetSwipeStartLocation _returnvalue_3)) ; The pressed event allows us to label the location of the users finger on the screen as the start of a possible swipe
      (bind _returnvalue_4 (Utilities|Time|SetTimerbyFunctionName 0 "StopMovement" (Variables|Default|GetPressCountDown))) ; TapTimer- if the released execution pin is not fired on the initial touch event before this timer counts down to 0, the input was a press, not a tap
      (Variables|Default|SetTapTimerHandle _returnvalue_4)
      (else
        (Development|PrintString "Hit Result Failed"))))
  (:Released
    (bind _output_get_2 (Variables|Default|SetSwipeCurrentLocation _returnvalue_3)) ; The released event gives us the location of their finger at the end of a possible swipe
    (if (> (Utilities|Time|GetTimerRemainingTimebyHandle (Variables|Default|GetTapTimerHandle)) 0.0) ; If the tap timer has time left remaining, the touch was a tap not a press
      (Utilities|Time|ClearandInvalidateTimerbyHandle (Variables|Default|GetTapTimerHandle)) ; This is neccessary to prepare the TapTimer for subsequent touches
      (bind _result (Math|Integer|IncrementInt (Variables|Default|GetTotalTaps))
        (:%20%20
          (Variables|Default|SetTotalTaps (Math|Integer|Clamp(Integer) _result 0 2))
          (Utilities|Time|ClearandInvalidateTimerbyHandle (Variables|Default|GetDoubleTapTimerHandle)) ; In the case of a Double Tap event, this will interrupt the DoubleTapTimer before it can reset the tap count to 0
          (bind _returnvalue_5 (Utilities|Time|SetTimerbyFunctionName 0 "ResetTapCount" (Variables|Default|GetDoubleTapCountDown))) ; DoubleTapTimer- if a second tap event is received before this timer counts down to 0, the touch was a Double Tap, not a Single Tap
          (Variables|Default|SetDoubleTapTimerHandle _returnvalue_5)
          (if (== (Variables|Default|GetTotalTaps) 1)
            (CallFunction|SingleTap)
            (elif (== (Variables|Default|GetTotalTaps) 2)
              (CallFunction|DoubleTap)))))
      (elif (>= (Math|Vector2D|Vector2DLength (- _output_get _output_get_2)) (Variables|Default|GetMinimumSwipeLength))
        (CallFunction|Swipe)
        (else
          (CallFunction|Press))))))

(fn ConstructionScript)

(fn MovetoLocation
  (params (Destination :type Vector) (Object%20Type :type Primitive%20Component%20Object%20Reference))
  ;[1 1 1] Moves the player to a location retrieved from the hit component we stored on touch input
  (Class|BPICrossControllerInterface|MovetoDestination(Message) (Variables|Default|GetAI_CON_REF) Destination (Variables|Default|GetAcceptanceRadius))
  (switch Utilities|FlowControl|Switch|SwitchonECollisionChannel (Collision|GetCollisionObjectType Object%20Type)
    (:ECC_GameTraceChannel2
      (Variables|Default|SetActionOnArrival "NewEnumerator3")
      (CallFunction|PollforEndOfMovement))
    (:ECC_GameTraceChannel3
      (Variables|Default|SetActionOnArrival "NewEnumerator2")
      (CallFunction|PollforEndOfMovement))
    (:ECC_GameTraceChannel4
      (Variables|Default|SetActionOnArrival "NewEnumerator0")
      (CallFunction|PollforEndOfMovement))
    (:ECC_GameTraceChannel6
      (Variables|Default|SetActionOnArrival "NewEnumerator1")
      (CallFunction|PollforEndOfMovement))))

(fn SetPlayerSpeed
  (params (Speed :type Float%20%28single-precision%29))
  (bind _player_char_ref (Variables|Default|GetPLAYER_CHAR_Ref))
  (bind _charactermovement (Variables|/Script/Engine.Character|GetCharacterMovement _player_char_ref))
  ;[1 1 1] If the players velocity is at or approaching run speed do nothing, otherwise assign the speed parameter to the players max walk speed
  (if (not (Math|Float|NearlyEqual(Float) (Math|Vector|VectorLength (Variables|/Script/Engine.MovementComponent|GetVelocity _charactermovement)) (Variables|Default|GetRunSpeed) 2e+02))
    (Variables|/Script/Engine.CharacterMovementComponent|SetMaxWalkSpeed _charactermovement Speed) ; Player is either standing still or walking, update their speed
  ))

(fn ResetTapCount
  (Variables|Default|SetTotalTaps 0))