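; Player controller for tap-to-move touch controls that classifies input as single tap, double tap, press or swipe.
; Touch-down caches a hit result and starts a timer; release uses timers, a tap count and drag length to pick the gesture.
; Single tap walks to the hit point via SimpleMoveToLocation or timeline-turns when on the pawn, double tap raises speed to run.
; Press stops movement; Swipe is an empty stub.
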(event Custom|SingleTap
  ;[1 1 1] Single Tap Event
  (if (Math|Vector|Equal(Vector) (Transformation|GetActorLocation (.HitActor (Collision|BreakHitResult (Variables|Default|GetHitResult)))) (Transformation|GetActorLocation (Pawn|GetControlledPawn)) 0.0001)
    (|QuickTurn) ; If the Touch input and the Player Character share the same location the Player Character does a 180 turn on the spot- NEEDS ANIMATION SET UP
    (else
      (CallFunction|SetPlayerSpeed (Variables|Default|GetSneakSpeed)) ; If not, then we want the player character to walk to the location of the Touch Input at walk speed
      (if (Variables|Default|GetHitResultIsValid)
        (CallFunction|MovetoLocation) ; Move the player to the location stored inside our HitComponent variable
        (Variables|Default|SetHitResultIsValid false)))))

(event Custom|Swipe
  ;[1 1 1] Swipe Event
)

(event Custom|Press
  ;[1 1 1] Press Event
  (AI|Navigation|StopMovement))

(event Custom|DoubleTap
  ;[1 1 1] Double Tap Event
  (CallFunction|SetPlayerSpeed (Variables|Default|GetRunSpeed)) ; On aDouble Tap we want the player character to run to the desired location. MoveToLocation was already called on the first tap, calling it a second time would risk changing the characters desired location, instead of just their speed
)

(event EventBeginPlay
  ;[1 1 1] Remove Virtual Joysticks from screen
  (Class|PlayerController|ActivateTouchInterface))

(event Input|TouchEvents|InputTouch
  (params (Location :type Vector) (FingerIndex :type ETouchIndex%20Enum))
  (bind _returnvalue (Game|GetPlayerController 0))
  (bind (_hitresult _returnvalue_2) (Class|PlayerController|GetHitResultUnderFingerbyChannel FingerIndex "TraceTypeQuery1" true))
  (bind (_locationx _locationy) (Class|PlayerController|GetInputTouchState _returnvalue "Touch1"))
  (bind _returnvalue_3 (Math|Vector2D|MakeVector2D _locationx _locationy))
  ;[1 1 1] Maps the possible Touch and Gesture Inputs with their corresponding Events
  (:Pressed
    (if _returnvalue_2
      (Variables|Default|SetHitResultIsValid _returnvalue_2)
      (Variables|Default|SetHitResult _hitresult)
      (bind _output_get (Variables|Default|SetSwipeStartLocation _returnvalue_3)) ; The pressed event allows us to label the location of the users finger on the screen as the start of a possible swipe
      (bind _returnvalue_4 (Utilities|Time|SetTimerbyFunctionName 0 "StopMovement" (Variables|Default|GetPressCountDown))) ; TapTimer- if the released execution pin is not fired on the initial touch event before this timer counts down to 0, the input was a press, not a tap
      (Variables|Default|SetTapTimerHandle _returnvalue_4)))
  (:Released
    (bind _output_get_2 (Variables|Default|SetSwipeCurrentLocation _returnvalue_3)) ; The released event gives us the location of their finger at the end of a possible swipe
    (if (> (Utilities|Time|GetTimerRemainingTimebyHandle (Variables|Default|GetTapTimerHandle)) 0.0) ; If the tap timer has time left remaining, the touch was a tap not a press
      (Utilities|Time|ClearandInvalidateTimerbyHandle (Variables|Default|GetTapTimerHandle)) ; This is neccessary to prepare the TapTimer for subsequent touches
      (bind _result (Math|Integer|IncrementInt (Variables|Default|GetTotalTaps))
        (:%20%20
          (Variables|Default|SetTotalTaps (Math|Integer|Clamp(Integer) _result 0 2))
          (Utilities|Time|ClearandInvalidateTimerbyHandle (Variables|Default|GetDoubleTapTimerHandle)) ; In the case of a Double Tap event, this will interrupt the DoubleTapTimer before it can reset the tap count to 0
          (bind _returnvalue_5 (Utilities|Time|SetTimerbyFunctionName 0 "ResetTapCount" (Variables|Default|GetDoubleTapCountDown))) ; DoubleTapTimer- if a second tap event is received before this timer counts down to 0, the touch was a Double Tap, not a Single Tap
          (Variables|Default|SetDoubleTapTimerHandle _returnvalue_5)
          (if (== (Variables|Default|GetTotalTaps) 1)
            (CallFunction|SingleTap)
            (elif (== (Variables|Default|GetTotalTaps) 2)
              (CallFunction|DoubleTap)))))
      (elif (>= (Math|Vector2D|Vector2DLength (- _output_get _output_get_2)) (Variables|Default|GetMinimumSwipeLength))
        (CallFunction|Swipe)
        (else
          (CallFunction|Press))))))

(fn ConstructionScript)

(fn MovetoLocation
  ;[1 1 1] Moves the player to a location retrieved from the hit component we stored on touch input
  (AI|Navigation|SimpleMovetoLocation self (.Location (Collision|BreakHitResult (Variables|Default|GetHitResult)))))

(fn SetPlayerSpeed
  (params (Speed :type Float%20%28single-precision%29))
  (bind _returnvalue (Game|GetPlayerCharacter 0))
  (bind _charactermovement (Variables|/Script/Engine.Character|GetCharacterMovement _returnvalue))
  ;[1 1 1] If the players velocity is at or approaching run speed do nothing, otherwise assign the speed parameter to the players max walk speed
  (if (not (Math|Float|NearlyEqual(Float) (Math|Vector|VectorLength (Variables|/Script/Engine.MovementComponent|GetVelocity _charactermovement)) (Variables|Default|GetRunSpeed) 2e+02))
    (Variables|/Script/Engine.CharacterMovementComponent|SetMaxWalkSpeed _charactermovement Speed) ; Player is either standing still or walking, update their speed
  ))

(fn ResetTapCount
  (Variables|Default|SetTotalTaps 0))